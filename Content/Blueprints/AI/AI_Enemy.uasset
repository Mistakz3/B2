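; AI_Enemy is an enemy that patrols waypoints, chases the player once seen and restarts the level when its capsule hits them.
; BeginPlay adds an audio component and starts a looping AIMoveTo patrol through the Waypoint array.
; PawnSensing sets PlayerSensed, which is never cleared here, and redirects movement to the player character.
; A capsule hit on a Player runs the RestartLevel console command.
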(event `self.PawnSensing.OnSeePawn`
  (params (Pawn :type "Pawn Object Reference"))
  (set `self.PlayerSensed` true)
  (`self.Follow Player`))

(event `FollowWaypoint`
  ;[1 1 1] Followplayer
  (`|AIMoveTo` self (0.0 0.0 0.0) (`|GetArrayItem` (`self.Waypoint`) (`self.CurrentWaypoint`))
    (:`OnSuccess`
      (`/Engine/EditorBlueprintResources/StandardMacros.IncrementInt` (`self.CurrentWaypoint`)
        (:`  `
          (if (>= (`self.CurrentWaypoint`) (`KismetArrayLibrary.Array_Length` (`self.Waypoint`)))
            (set `self.CurrentWaypoint` 0))
          (`self.FollowWaypoint`))))))

(event `Follow Player`
  (if (`self.PlayerSensed`)
    (`|AIMoveTo` self (0.0 0.0 0.0) (`GameplayStatics.GetPlayerCharacter` 0))
    (else
      (`KismetSystemLibrary.RetriggerableDelay` 1.0)
      (`self.FollowWaypoint`))))

(event `self.ReceiveBeginPlay`
  ;[1 1 1] Followplayer
  (`|ExecutionSequence`
    (:`then_0`
      (`self.FollowWaypoint`))
    (:`then_1`
      (`AddComponent|NODE_AddAudioComponent-0`))))

(event `self.CapsuleComponent.OnComponentHit`
  (params (HitComponent :type "PrimitiveComponent Object Reference") (OtherActor :type "Actor Object Reference") (OtherComp :type "PrimitiveComponent Object Reference") (NormalImpulse :type "Vector Structure") (Hit :type "HitResult Structure (by ref)"))
  ;[1 1 1] PlayerDeath
  (cast `/Game/Blueprints/Player_Character/Player` OtherActor)
  (`KismetSystemLibrary.ExecuteConsoleCommand` "RestartLevel" null))

(fn `UserConstructionScript`)