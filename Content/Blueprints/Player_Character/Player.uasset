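; Player character Blueprint that handles movement, looking, jumping, a toggleable torch and a basic pickup action.
; Input axes drive forward and strafe movement plus controller yaw and pitch, and a FlipFlop switches the SpotLight's visibility.
; Pressing E checks overlapping Pickup actors for the Pick interface and adds a skeletal mesh component to the player for each match, without calling the interface or altering the item.
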(event `Key|E`
  (params (Key :type "Key Structure"))
  ;[1 1 1] Pickup
  (:`Pressed`
    (for _array_element (`self.GetOverlappingActors` "/Game/Blueprints/Player_Character/Pickup.Pickup_C")
      (if (`KismetSystemLibrary.DoesImplementInterface` _array_element "/Game/Blueprints/Player_Character/Pick.Pick_C")
        (`AddComponent|NODE_AddSkeletalMeshComponent-1`)))))

(event `InputAxis|MoveForward`
  (params (AxisValue :type "Float (single-precision)"))
  ;[1 1 1] Character Movement
  (`self.AddMovementInput` (`self.GetActorForwardVector`) AxisValue))

(event `InputAxis|MoveRight`
  (params (AxisValue :type "Float (single-precision)"))
  ;[1 1 1] Character Movement
  (`self.AddMovementInput` (`self.GetActorRightVector`) AxisValue))

(event `InputAction|On/Off`
  (params (Key :type "Key Structure"))
  (bind _spotlight (`self.SpotLight`))
  ;[1 1 1] Torch
  (:`Pressed`
    (`/Engine/EditorBlueprintResources/StandardMacros.FlipFlop`
      (:`A`
        (`SceneComponent.SetVisibility` _spotlight true false))
      (:`B`
        (`SceneComponent.SetVisibility` _spotlight false false)))))

(event `InputAxis|Turn`
  (params (AxisValue :type "Float (single-precision)"))
  ;[1 1 1] Character Movement
  (`self.AddControllerYawInput` AxisValue))

(event `InputAxis|LookUp`
  (params (AxisValue :type "Float (single-precision)"))
  ;[1 1 1] Character Movement
  (`self.AddControllerPitchInput` AxisValue))

(event `InputAction|Jump`
  (params (Key :type "Key Structure"))
  (:`Pressed`
    (`self.Jump`)))

(fn `UserConstructionScript`)