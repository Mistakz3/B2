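; Cross pickup actor that counts toward the player's win and ends the game when collected.
; When a Player overlaps its Box, it increments that player's PickupNumber, prints the count and destroys itself.
; Once the count is at least one, so on the first pickup, it shows the WinCondition widget and pauses the game.
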(event `self.Box.OnComponentBeginOverlap`
  (params (OverlappedComponent :type "PrimitiveComponent Object Reference") (OtherActor :type "Actor Object Reference") (OtherComp :type "PrimitiveComponent Object Reference") (OtherBodyIndex :type Integer) (bFromSweep :type Boolean) (SweepResult :type "HitResult Structure (by ref)"))
  (bind _asplayer (cast `/Game/Blueprints/Player_Character/Player` OtherActor))
  (bind _pickupnumber (`/Game/Blueprints/Player_Character/Player.PickupNumber` _asplayer))
  (bind _output_get (set `/Game/Blueprints/Player_Character/Player.PickupNumber` (+ _pickupnumber 1) _asplayer))
  (`KismetSystemLibrary.PrintString` (`KismetStringLibrary.Conv_IntToString` _output_get))
  (`self.K2_DestroyActor`)
  (if (>= _pickupnumber 1)
    (bind _returnvalue (`|CreateWidget` "/Game/Blueprints/Gameplay_Winning/WinCondition.WinCondition_C"))
    (`UserWidget.AddToViewport` _returnvalue 0)
    (`GameplayStatics.SetGamePaused` true)))

(fn `UserConstructionScript`)