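; BP_InteractableBase is a base Blueprint for interactable objects, with child classes overriding OnInteract to add their behavior.
; Interact applies the interact-once and cooldown rules by clearing ActiveForInteract, then calls OnInteract.
; A cooldown sets a timer by function name that runs ResetInteract, re-enabling the object even if it is marked interact-once.
; Getters expose active state, interaction type, prompt, sound, location, hold duration, tap count and both rules.
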(event `/Game/InteractionSystem/Interfaces/BPI_Interactable.Interact`
  (params (Interactor :type "Actor Object Reference"))
  (`|ExecutionSequence`
    (:`then_0`
      (`self.CheckInteractOnce`))
    (:`then_1`
      (`self.CheckInteractionCooldown`))
    (:`then_2`
      (`self.ONINteract`))))

(event `OnInteract`
  ; override this in childs
)

(fn `CheckInteractionCooldown`
  (if (> (`self.InteractionCooldown`) 0.0)
    (set `self.ActiveForInteract` false)
    (`KismetSystemLibrary.K2_SetTimer` null "ResetInteract" (`self.InteractionCooldown`))))

(fn `CheckInteractOnce`
  (if (`self.InteractOnce?`)
    (set `self.ActiveForInteract` false)))

(fn `GetActiveForInteract`
  (returns (Value :type Boolean))
  (return (`self.ActiveForInteract`)))

(fn `GetHoldDuration`
  (returns (Duration :type "Float (double-precision)"))
  (return (`self.HoldDuration`)))

(fn `GetInteractionCooldown`
  (returns (Cooldown :type "Float (double-precision)"))
  (return (`self.InteractionCooldown`)))

(fn `GetInteractionLocation`
  (returns (Location :type "Vector Structure"))
  (return (`SceneComponent.K2_GetComponentLocation` (`self.InteractionLocation`))))

(fn `GetInteractionPrompt`
  (returns (Prompt :type Text))
  (return (`self.InteractionAffix`)))

(fn `GetInteractionSound`
  (returns (Sound :type "SoundBase Object Reference"))
  (return (`self.InteractionSound`)))

(fn `GetInteractionType`
  (returns (Type :type "/Game/InteractionSystem/Enums/E_InteractionType Enum"))
  (return (`self.InteractionType`)))

(fn `GetInteractOnce`
  (returns (Value :type Boolean))
  (return (`self.InteractOnce?`)))

(fn `GetTapCount`
  (returns (Value :type Integer))
  (return (`self.TapCount`)))

(fn `ResetInteract`
  (set `self.ActiveForInteract` true))

(fn `UserConstructionScript`)