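; BP_Door is an interactable preset for a hinged door that toggles open and closed on each interaction.
; The interact event runs a FlipFlop that alternates between the OpenDoor and CloseDoor events, which play or reverse the Door timeline.
; Each timeline update lerps the static mesh's relative yaw between closed and a quarter turn open.
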(event `self.ONINteract`
  (`/Engine/EditorBlueprintResources/StandardMacros.FlipFlop`
    (:`A`
      (`self.OpenDoor`))
    (:`B`
      (`self.CloseDoor`))))

(event `OpenDoor`
  (bind (_direction _alpha) (`Timeline|Door` :!label _label)
    (:`Update`
      (`SceneComponent.K2_SetRelativeRotation` (`self.StaticMesh`) (`KismetMathLibrary.MakeRotator` 0.0 0.0 (`KismetMathLibrary.Lerp` 0.0 -90.0 _alpha)) false false))))

(event `CloseDoor`
  (goto _label :!via `Reverse`))

(fn `UserConstructionScript`
  (`parent.UserConstructionScript`))